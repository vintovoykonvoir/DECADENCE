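; Automatic hinged door actor that swings open when a Character enters its Box1 trigger and closes when one leaves.
; On begin overlap, the dot product of the character's forward vector and the root's forward vector picks the swing direction from the character's facing.
; Timeline_0 drives a yaw lerp on the Door component toward a quarter turn either way, and end overlap reverses the timeline.
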(event OnComponentBeginOverlap(Box1)
  (params (OverlappedComponent :type Primitive%20Component%20Object%20Reference) (OtherActor :type Actor%20Object%20Reference) (OtherComp :type Primitive%20Component%20Object%20Reference) (OtherBodyIndex :type Integer) (bFromSweep :type Boolean) (SweepResult :type Hit%20Result%20Structure%20%28by%20ref%29))
  (bind _ascharacter (Utilities|Casting|CastToCharacter OtherActor))
  (Variables|Default|SetWherePlayer (>= (Math|Vector|DotProduct (Transformation|GetActorForwardVector _ascharacter) (Math|Vector|GetForwardVector (Variables|Default|GetDefaultSceneRoot))) 0.0))
  (bind _rotz (Timeline|Timeline_0 Play)
    (:Update
      (if (Variables|Default|GetWherePlayer)
        (Transformation|SetRelativeLocationAndRotation (Variables|Default|GetDoor) "0, 0, 0" (Math|Rotator|MakeRotator 0.0 0.0 (Math|Float|Lerp 0.0 -9e+01 _rotz)) false false)
        (else
          (Transformation|SetRelativeLocationAndRotation (Variables|Default|GetDoor) "0, 0, 0" (Math|Rotator|MakeRotator 0.0 0.0 (Math|Float|Lerp 0.0 9e+01 _rotz)) false false))))))

(event OnComponentEndOverlap(Box1)
  (params (OverlappedComponent :type Primitive%20Component%20Object%20Reference) (OtherActor :type Actor%20Object%20Reference) (OtherComp :type Primitive%20Component%20Object%20Reference) (OtherBodyIndex :type Integer))
  (Utilities|Casting|CastToCharacter OtherActor)
  (bind _rotz (Timeline|Timeline_0 Reverse)
    (:Update
      (if (Variables|Default|GetWherePlayer)
        (Transformation|SetRelativeLocationAndRotation (Variables|Default|GetDoor) "0, 0, 0" (Math|Rotator|MakeRotator 0.0 0.0 (Math|Float|Lerp 0.0 -9e+01 _rotz)) false false)
        (else
          (Transformation|SetRelativeLocationAndRotation (Variables|Default|GetDoor) "0, 0, 0" (Math|Rotator|MakeRotator 0.0 0.0 (Math|Float|Lerp 0.0 9e+01 _rotz)) false false))))))

(fn ConstructionScript)