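; BP_BaseDoor is a base door that loads another level when interacted with.
; On BeginPlay it caches the BP_BaseGameInstance.
; Interacting stores the player's location and rotation in that game instance and sets IsMoveDoor to false.
; After a short delay it opens the level named by DoorLevel, so the saved values persist across the level change.
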(event EventInteracteble
  (params (Player :type Character%20Object%20Reference))
  (Variables|Default|SetPlayer Player)
  (|SetLastLocationAndRotation)
  (Utilities|FlowControl|Delay 0.2)
  (Game|OpenLevel(byName) (Variables|Default|GetDoorLevel)))

(event EventBeginPlay
  ;[1 1 1] EventBeginPlay
  (bind _asbp_base_game_instance (Utilities|Casting|CastToBP_BaseGameInstance (Game|GetGameInstance)))
  (Variables|Default|SetAs%20BP%20Base%20Game%20Instance _asbp_base_game_instance))

(fn ConstructionScript)