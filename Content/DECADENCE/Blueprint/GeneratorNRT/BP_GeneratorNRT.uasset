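; BP_GeneratorNRT is an interactable generator that produces NTR for the player's inventory.
; On interact it casts the player to ThirdPersonCharacter, waits TimeGeneration, increments the inventory component's NTR count and shows the new total on the HUD.
; The CanCreate flag blocks overlapping requests until a short delay after creation, and stays false if the cast fails.
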(event EventInteracteble
  (params (Player :type Character%20Object%20Reference))
  (if (Variables|Default|GetCanCreate)
    (Variables|Default|SetCanCreate false)
    (bind _asthird_person_character (Utilities|Casting|CastToThirdPersonCharacter Player))
    (Utilities|FlowControl|Delay (Variables|Default|GetTimeGeneration))
    (bind _result (Math|Integer|IncrementInt (Variables|/Game/DECADENCE/Blueprint/Character/Component/BP_CharacterInventoryComponent.BP_CharacterInventoryComponent_C|GetNTR (Variables|/Game/DECADENCE/Blueprint/Character/ThirdPersonCharacter.ThirdPersonCharacter_C|GetBP_CharacterInventoryComponent _asthird_person_character)))
      (:%20%20
        (bind _output_get (Variables|/Game/DECADENCE/Blueprint/Character/Component/BP_CharacterInventoryComponent.BP_CharacterInventoryComponent_C|SetNTR (Variables|/Game/DECADENCE/Blueprint/Character/ThirdPersonCharacter.ThirdPersonCharacter_C|GetBP_CharacterInventoryComponent _asthird_person_character) _result))
        (Default|EventInfoMess (Variables|/Game/DECADENCE/Blueprint/Character/ThirdPersonCharacter.ThirdPersonCharacter_C|GetHUD _asthird_person_character) (Utilities|Text|ToText(String) (Utilities|String|Append "Create NTR" ":" (Utilities|String|ToString(Integer) _output_get))))
        (Utilities|FlowControl|Delay 0.5)
        (Variables|Default|SetCanCreate true)))))

(fn ConstructionScript)