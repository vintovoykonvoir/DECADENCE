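; BP_PointNrt is an interactable point that replaces itself with a spawned BP_Nrt actor, with toggleable in-world and minimap marker widgets hidden at BeginPlay.
; While IsWork is set, its box overlap registers it as the ThirdPersonCharacter's InteractActor, cleared on exit.
; Interacting spawns BP_Nrt at the Scene component's transform after CheckNTR passes, then destroys the point.
; CheckNTR's inventory NTR count comparison is left unconnected.
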(event OnComponentBeginOverlap(Box)
  (params (OverlappedComponent :type Primitive%20Component%20Object%20Reference) (OtherActor :type Actor%20Object%20Reference) (OtherComp :type Primitive%20Component%20Object%20Reference) (OtherBodyIndex :type Integer) (bFromSweep :type Boolean) (SweepResult :type Hit%20Result%20Structure%20%28by%20ref%29))
  ;[1 1 1] Comment
  (if (Variables|Default|GetIsWork)
    (bind _asthird_person_character (Utilities|Casting|CastToThirdPersonCharacter OtherActor))
    (bind _output_get (Variables|Default|SetPlayer _asthird_person_character))
    (Variables|/Game/DECADENCE/Blueprint/Character/ThirdPersonCharacter.ThirdPersonCharacter_C|SetInteractActor _output_get self)
    (Variables|/Game/DECADENCE/Blueprint/Character/ThirdPersonCharacter.ThirdPersonCharacter_C|SetIsTrigger _output_get true)))

(event OnComponentEndOverlap(Box)
  (params (OverlappedComponent :type Primitive%20Component%20Object%20Reference) (OtherActor :type Actor%20Object%20Reference) (OtherComp :type Primitive%20Component%20Object%20Reference) (OtherBodyIndex :type Integer))
  ;[1 1 1] Comment
  (bind _asthird_person_character (Utilities|Casting|CastToThirdPersonCharacter OtherActor))
  (Variables|/Game/DECADENCE/Blueprint/Character/ThirdPersonCharacter.ThirdPersonCharacter_C|SetInteractActor _asthird_person_character 0)
  (Variables|Default|SetPlayer 0)
  (Variables|/Game/DECADENCE/Blueprint/Character/ThirdPersonCharacter.ThirdPersonCharacter_C|SetIsTrigger _asthird_person_character false))

(event Custom|SpawnNrt
  (bind _scene (Variables|Default|GetScene))
  ;[1 1 1] Comment
  (Game|SpawnActorfromClass "/Game/DECADENCE/Blueprint/Nrt/BP_Nrt.BP_Nrt_C" (Math|Transform|MakeTransform (Transformation|GetWorldLocation _scene) (Transformation|GetWorldRotation _scene) "1,1,1") "Undefined" 0 0)
  (Development|PrintString "Out"))

(event Custom|ActivatePoint
  (params (bPropagateToChildren :type Boolean))
  ;[1 1 1] ActivatePointInCharacter
  (Rendering|SetVisibility (Variables|Default|GetWidget) bPropagateToChildren false))

(event Custom|ActivatePointInMinimap
  (params (bNewVisibility :type Boolean))
  ;[1 1 1] ActivatePointInMinimap
  (Rendering|SetVisibility (Variables|Default|GetWidget1) bNewVisibility false))

(event EventBeginPlay
  ;[1 1 1] Begin Play: Deactivate Point
  (CallFunction|ActivatePoint false)
  (CallFunction|ActivatePointinMinimap false))

(event EventInteracteble
  (params (Player :type Character%20Object%20Reference))
  ;[1 1 1] Comment
  (if (|CheckNTR Player)
    (Utilities|FlowControl|Delay 0.2)
    (CallFunction|SpawnNrt)
    (Utilities|FlowControl|Delay 0.2)
    (Actor|DestroyActor)))

(fn ConstructionScript)