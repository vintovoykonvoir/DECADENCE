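; Base computer actor that the player toggles in and out of using through a FlipFlop on interaction.
; Entering blends the view to the computer, shows the cursor, disables movement, hides the HUD and calls the character's SetDateHours; leaving reverses the view, cursor, movement and HUD changes.
; A separate SetDate/Hours function formats the time and date from the target's inventory component into the WG_Computer widget's down panel.
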(event Custom|CameraIn
  (params (Character :type Character%20Object%20Reference))
  ;[1 1 1] CameraIn
  (Game|Player|SetViewTargetwithBlend (Game|GetPlayerController 0) Character 0.0 "VTBlend_EaseIn" 1.0 false)
  (Variables|/Script/Engine.PlayerController|SetbShowMouseCursor (Game|GetPlayerController 0) false)
  (Pawn|Components|CharacterMovement|SetMovementMode (Variables|/Script/Engine.Character|GetCharacterMovement Character) "MOVE_Walking" 0)
  (Widget|SetVisibility (Variables|/Game/DECADENCE/Blueprint/Character/ThirdPersonCharacter.ThirdPersonCharacter_C|GetHUD (.AsThird%20Person%20Character (Utilities|Casting|CastToThirdPersonCharacter Character))) "Visible"))

(event Custom|CameraOut
  (params (Character :type Character%20Object%20Reference))
  (bind _asthird_person_character (Utilities|Casting|CastToThirdPersonCharacter Character))
  ;[1 1 1] CameraOut
  (Game|Player|SetViewTargetwithBlend (Game|GetPlayerController 0) self 0.0 "VTBlend_EaseOut" 1.0 false)
  (Variables|/Script/Engine.PlayerController|SetbShowMouseCursor (Game|GetPlayerController 0) true)
  (Pawn|Components|CharacterMovement|SetMovementMode (Variables|/Script/Engine.Character|GetCharacterMovement Character) "MOVE_None" 0)
  (Widget|SetVisibility (Variables|/Game/DECADENCE/Blueprint/Character/ThirdPersonCharacter.ThirdPersonCharacter_C|GetHUD _asthird_person_character) "Hidden")
  (|SetDate/Hours _asthird_person_character)
  (bind _aswg_computer (Utilities|Casting|CastToWG_Computer (UserInterface|GetWidget (Variables|Default|GetWidget)))))

(event EventInteracteble
  (params (Player :type Character%20Object%20Reference))
  (Utilities|FlowControl|FlipFlop
    (:A
      (CallFunction|CameraOut Player))
    (:B
      (CallFunction|Camerain Player))))

(fn ConstructionScript)